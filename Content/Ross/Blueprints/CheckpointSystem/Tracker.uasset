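; Race manager for a lap-based checkpoint time trial, passing map settings, medal times and save slot to the CheckpointPlayerController.
; It numbers the checkpoint list, activates each in sequence, counts laps and updates the respawn point until the race completes.
; A Timeline serves as the split timer, and each clear briefly shows a comparison against that checkpoint's saved time.
; At race end, it ranks the player against six preset leaderboard times.
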(event `self.ReceiveBeginPlay`
  ;[1 1 1] BeginPlay // Get controller reference // Game init
  (bind _ascheckpoint_player_controller (cast `/Game/Ross/Blueprints/CheckpointSystem/CheckpointPlayerController` (`GameplayStatics.GetPlayerController` 0)))
  (set `self.ControllerReference` _ascheckpoint_player_controller)
  (`self.InitLeaderboard`)
  (`self.ApplySettings`)
  (`self.StartSequence`)
  (`self.StartCheckpointTimer`)
  (bind _ascheckpoint_player_controller_2 (cast `/Game/Ross/Blueprints/CheckpointSystem/CheckpointPlayerController` (`GameplayStatics.GetPlayerController` 0)))
  (set `/Game/Ross/Blueprints/CheckpointSystem/CheckpointPlayerController.TrackerReference` self _ascheckpoint_player_controller_2)
  (set `self.ComparisonShow` "Hidden"))

(event `ApplySettings`
  (bind _controllerreference (`self.ControllerReference`))
  ;[1 1 1] Apply user settings on startup
  (set `/Game/Ross/Blueprints/CheckpointSystem/CheckpointPlayerController.MaxLaps` (`self.MaxLaps`) _controllerreference)
  (`self.UpdateTimes`)
  (`/Game/Ross/Blueprints/CheckpointSystem/CheckpointPlayerController.StartGameSetup` _controllerreference)
  (set `/Game/Ross/Blueprints/CheckpointSystem/CheckpointPlayerController.SaveSlot` (`self.SaveGameName`) _controllerreference)
  (set `/Game/Ross/Blueprints/CheckpointSystem/CheckpointPlayerController.NameOfMap` (`self.NameOfMap`) _controllerreference))

(event `RaceEnded`
  ;[1 1 1] Leaderboard
  (`|ExecutionSequence`
    (:`then_0`
      (for (_array_element _array_index) (`self.LeaderboardTimes`)
        (if (> _array_element (`/Game/Ross/Blueprints/CheckpointSystem/CheckpointPlayerController.ActualRaceTime` (`self.ControllerReference`)))
          (set `self.FoundPlacement` true)
          (set `self.PlayerPlacement` (+ _array_index (`self.PlayerPlacement`) 1))
          (break))))
    (:`then_1`
      (for _array_element_2 (`self.LeaderboardTimes`)
        (`KismetArrayLibrary.Array_Add` (`self.PlacementTimeText`) (`/Game/Ross/Blueprints/CheckpointSystem/TimeConversion.TimeToText` _array_element_2)))
      (set `self.FirstPlaceTimeText` (`|GetArrayItem` (`self.PlacementTimeText`)))
      (set `self.SecondPlaceTimeText` (`|GetArrayItem` (`self.PlacementTimeText`) 1))
      (set `self.ThirdPlaceTimeText` (`|GetArrayItem` (`self.PlacementTimeText`) 2))
      (set `self.FourthPlaceTimeText` (`|GetArrayItem` (`self.PlacementTimeText`) 3))
      (set `self.FifthPlaceTimeText` (`|GetArrayItem` (`self.PlacementTimeText`) 4))
      (set `self.SixthPlaceTimeText` (`|GetArrayItem` (`self.PlacementTimeText`) 5)))))

(event `StartCheckpointTimer`
  ;[1 1 1] Checkpoint timer
  (bind (_direction _time) (`Timeline|CheckpointTImer` :!via `PlayFromStart` :!label _label)
    (:`Update`
      (set `self.LocalCheckpointTime` _time))))

(event `StopCheckpointTimer`
  ;[1 1 1] Checkpoint timer
  (goto _label :!via `Stop`))

(event `InitLeaderboard`
  ;[1 1 1] Initialize leaderboard
  (`KismetArrayLibrary.Array_Add` (`self.LeaderboardTimes`) (`self.FirstPlaceTime`))
  (`KismetArrayLibrary.Array_Add` (`self.LeaderboardTimes`) (`self.SecondPlaceTime`))
  (`KismetArrayLibrary.Array_Add` (`self.LeaderboardTimes`) (`self.ThirdPlaceTime`))
  (`KismetArrayLibrary.Array_Add` (`self.LeaderboardTimes`) (`self.FourthPlaceTime`))
  (`KismetArrayLibrary.Array_Add` (`self.LeaderboardTimes`) (`self.FifthPlaceTime`))
  (`KismetArrayLibrary.Array_Add` (`self.LeaderboardTimes`) (`self.SixthPlaceTime`)))

(event `StartSequence`
  (bind _checkpointslist (`self.CheckpointsList`))
  ;[1 1 1] Startup // Gets all checkpoints, activates first checkpoint, binds event to checkpoint cleared
  (for (_array_element _array_index) _checkpointslist
    (set `/Game/Ross/Blueprints/CheckpointSystem/Checkpoint.CheckpointNumber` (+ _array_index 1) _array_element))
  (set `self.TotalCheckpoints` (`KismetArrayLibrary.Array_Length` _checkpointslist))
  (`self.ActivateCheckpoint` (`|GetArrayItem` _checkpointslist))
  ;;[1 1 1] Potentially need to move this to loop body
  (for _array_element_2 (`self.CheckpointsList`)
    (add `/Game/Ross/Blueprints/CheckpointSystem/Checkpoint.CheckpointCleared` _array_element_2 (delegate `CheckpointCleared`))))

(event `CheckpointCleared`
  (params (NextCheckpoint :type Integer))
  (bind _controllerreference (`self.ControllerReference`))
  ;[1 1 1] Checkpoint cleared - check to see if race is over, if so restart
  (set `self.ComparisonTime` (- (`/Game/Ross/Blueprints/CheckpointSystem/CheckpointPlayerController.ActualRaceTime` (`self.ControllerReference`)) (`/Game/Ross/Blueprints/CheckpointSystem/Checkpoint.SavedTime` (`|GetArrayItem` (`self.CheckpointsList`) (- NextCheckpoint 1)))))
  (`|ExecutionSequence`
    (:`then_0`
      (`self.LapCheck` NextCheckpoint)
      (if (`/Game/Ross/Blueprints/CheckpointSystem/CheckpointPlayerController.RaceComplete` _controllerreference)
        (`/Game/Ross/Blueprints/CheckpointSystem/CheckpointPlayerController.EndRaceSequence` _controllerreference)))
    (:`then_1`
      (set `self.ComparisonShow` "Visible")
      (`KismetSystemLibrary.Delay` 3.0)
      (set `self.ComparisonShow` "Hidden"))))

(fn `ActivateCheckpoint`
  (params (NextCheckpoint :type "/Game/Ross/Blueprints/CheckpointSystem/Checkpoint Object Reference"))
  (bind _trigger (`/Game/Ross/Blueprints/CheckpointSystem/Checkpoint.Trigger` NextCheckpoint))
  ;[1 1 1] Activates next checkpoint
  (`SceneComponent.SetHiddenInGame` _trigger false false)
  (set `PrimitiveComponent.bGenerateOverlapEvents` true _trigger))

(fn `LapCheck`
  (params (Checkpoint :type Integer))
  (locals (LocalCheckpoint :type Integer))
  ;[1 1 1] LapCheck script // Checks to see if a lap has been complete or sets up next checkpoint
  (bind _output_get (set `local.LocalCheckpoint` Checkpoint))
  (if (== _output_get (`self.TotalCheckpoints`))
    (bind _isracecomplete (`self.RaceCompleteCheck`))
    (if (not _isracecomplete)
      (`self.ActivateCheckpoint` (`|GetArrayItem` (`self.CheckpointsList`))))
    (`/Game/Ross/Blueprints/CheckpointSystem/CheckpointPlayerController.UpdateLap` (`self.ControllerReference`))
    (`self.RaceFinished`)
    (else
      (`self.ActivateCheckpoint` (`|GetArrayItem` (`self.CheckpointsList`) (`local.LocalCheckpoint`)))
      (`self.StopCheckpointTimer`)
      (set `/Game/Ross/Blueprints/CheckpointSystem/Checkpoint.TimeAtPass` (`self.LocalCheckpointTime`) (`|GetArrayItem` (`self.CheckpointsList`) (`local.LocalCheckpoint`)))
      (`self.StartCheckpointTimer`)))
  (set `/Game/Ross/Blueprints/CheckpointSystem/CheckpointPlayerController.RespawnLocation` (`self.GetTransform` (`|GetArrayItem` (`self.CheckpointsList`) (- (`local.LocalCheckpoint`) 1))) (`self.ControllerReference`)))

(fn `RaceCompleteCheck`
  (returns (IsRaceComplete :type Boolean))
  (locals (LocalComplete :type Boolean))
  (bind _controllerreference (`self.ControllerReference`))
  (bind _controllerreference_2 (`self.ControllerReference`))
  ;[1 1 1] Race complete check // Sets race complete in checkpoint controller
  (if (>= (`/Game/Ross/Blueprints/CheckpointSystem/CheckpointPlayerController.ActualLap` _controllerreference) (`/Game/Ross/Blueprints/CheckpointSystem/CheckpointPlayerController.MaxLaps` _controllerreference))
    (bind _output_get (set `/Game/Ross/Blueprints/CheckpointSystem/CheckpointPlayerController.RaceComplete` true _controllerreference_2))
    (set `local.LocalComplete` _output_get)
    (else
      (bind _output_get_2 (set `/Game/Ross/Blueprints/CheckpointSystem/CheckpointPlayerController.RaceComplete` false _controllerreference_2))
      (set `local.LocalComplete` _output_get_2)))
  (return (`local.LocalComplete`)))

(fn `UpdateTimes`
  (bind _controllerreference (`self.ControllerReference`))
  ;[1 1 1] Pass user times to checkpoint player controller times
  (set `/Game/Ross/Blueprints/CheckpointSystem/CheckpointPlayerController.GoldTime` (`self.GoldTIme`) _controllerreference)
  (set `/Game/Ross/Blueprints/CheckpointSystem/CheckpointPlayerController.SilverTime` (`self.SilverTime`) _controllerreference)
  (set `/Game/Ross/Blueprints/CheckpointSystem/CheckpointPlayerController.BronzeTime` (`self.BronzeTime`) _controllerreference)
  (set `/Game/Ross/Blueprints/CheckpointSystem/CheckpointPlayerController.DefaultBestLapTime` (`self.DefaultBestLap`) _controllerreference)
  (set `/Game/Ross/Blueprints/CheckpointSystem/CheckpointPlayerController.DefaultBestRaceTime` (`self.DefaultBestTime`) _controllerreference))

(fn `UserConstructionScript`)