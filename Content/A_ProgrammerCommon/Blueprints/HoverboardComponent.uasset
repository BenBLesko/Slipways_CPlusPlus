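; Player hoverboard actor that drives speed, boost, pickups, hazards, Wwise audio and checkpoint respawning.
; Tick pushes the physics cube using the acceleration component, with pseudo-gravity along averaged hover-ray normals when grounded, or straight down when airborne.
; The visible board's tilt lags the cube, which self-levels in air and has clamped roll.
; Boosts, overcharge, landings and lava adjust speed or camera FOV; boost drain and flip-respawn logic are disconnected.
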(event `self.ReceiveBeginPlay`
  ;[1 1 1] Initializes the Hover Components using the Board's Mesh
  (`/Game/A_ProgrammerCommon/Blueprints/HoverComponent.InitComponent` (`self.HoverComponent`) (`self.Cube`))
  (`/Game/A_ProgrammerCommon/Blueprints/HoverComponent.InitComponent` (`self.HoverComponent1`) (`self.Cube`))
  (`/Game/A_ProgrammerCommon/Blueprints/HoverComponent.InitComponent` (`self.HoverComponent2`) (`self.Cube`))
  (`/Game/A_ProgrammerCommon/Blueprints/HoverComponent.InitComponent` (`self.HoverComponent3`) (`self.Cube`))
  (`/Game/Micheal/Blueprints/JumpComponent.Init Component` (`self.JumpComponent`) (`self.Cube`) (`self.jumpForce`))
  (`/Game/Micheal/Blueprints/AccelerationComponent.Init Component` (`self.AccelerationComponent`) (`self.Cube`) (`self.Camera`))
  (`/Game/Ross/Blueprints/InAirComponent.Init Component` (`self.InAirComponent`) (`self.Cube`) (`self.Sphere`))
  (`/Game/A_ProgrammerCommon/Blueprints/HoverComponent.InitComponent` (`self.UpComponent`) (`self.Cube`))
  (bind _ascheckpoint_player_controller (cast `/Game/Ross/Blueprints/CheckpointSystem/CheckpointPlayerController` (`GameplayStatics.GetPlayerController` 0)))
  (bind _output_get (set `self.CheckpointControllerReference` _ascheckpoint_player_controller))
  (set `/Game/Ross/Blueprints/CheckpointSystem/CheckpointPlayerController.RespawnLocation` (`self.GetTransform`) _output_get)
  (`/Game/Ross/Blueprints/HoverboardMovement/Turning.InitComponent` (`self.Turning`) self)
  (`/Game/Micheal/Blueprints/SmoothCornerRaycast.InitComponent` (`self.SmoothCornerRaycast`) self)
  (`self.Regen Boost`)
  (`/Game/Tony/Animation/LandingStre.InitComponent` (`self.LandingStre`) self)
  (`self.WwiseSetup`)
  (`KismetArrayLibrary.Array_Add` (`self.HoverComponentArray`) (`self.HoverComponent`))
  (`KismetArrayLibrary.Array_Add` (`self.HoverComponentArray`) (`self.HoverComponent1`))
  (`KismetArrayLibrary.Array_Add` (`self.HoverComponentArray`) (`self.HoverComponent2`))
  (`KismetArrayLibrary.Array_Add` (`self.HoverComponentArray`) (`self.HoverComponent3`)))

(event `self.ReceiveTick`
  (params (DeltaSeconds :type "Float (single-precision)"))
  (bind _isovercharging (`self.isOvercharging`))
  (bind _accelerationcomponent (`self.AccelerationComponent`))
  (bind _isboosting (`self.isBoosting`))
  (bind _returnvalue (`SceneComponent.K2_GetComponentRotation` (`self.Cube`)))
  (bind (_returnvalue_x _returnvalue_y _returnvalue_z) (`KismetMathLibrary.BreakVector` (`SceneComponent.K2_GetComponentLocation` (`self.Cube`))))
  (bind _returnvalue_2 (`SceneComponent.K2_GetComponentRotation` (`self.boardMesh`)))
  (bind (_relativerotation_roll _relativerotation_pitch _relativerotation_yaw) (`KismetMathLibrary.BreakRotator` (`SceneComponent.RelativeRotation` (`self.Cube`))))
  (bind _acceleration (`/Game/Micheal/Blueprints/AccelerationComponent.Acceleration` (`self.AccelerationComponent`)))
  (bind (_returnvalue_roll _returnvalue_pitch) (`KismetMathLibrary.BreakRotator` (`KismetMathLibrary.RInterpTo` _returnvalue_2 _returnvalue (`self.Delta Seconds`) (`self.Roll Speed`))))
  (bind _returnvalue_roll_2 (`KismetMathLibrary.BreakRotator` (`KismetMathLibrary.RInterpTo` _returnvalue_2 _returnvalue (`self.Delta Seconds`) (`self.Pitch Speed`))))
  ;[1 1 1] Check the speed and slow down the Hoverboard when not touching ground
  (set `self.Delta Seconds` DeltaSeconds)
  (`|ExecutionSequence`
    (:`then_0`
      (bind _astimer_hud (cast `/Game/Micheal/Blueprints/timerHUD` (`PlayerController.GetHUD` (`GameplayStatics.GetPlayerController` 0))))
      (`self.Accelerate`)
      (set `self.Tony Acceleration` _acceleration)
      (`/Game/Micheal/Blueprints/TimerUI.Set Speed` (`/Game/Micheal/Blueprints/timerHUD.Timer UI` _astimer_hud) _acceleration)
      (bind _grounddetected (`self.GroundCheck`))
      (`/Game/Micheal/Blueprints/JumpComponent.OnGround` (`self.JumpComponent`) _grounddetected)
      (`/Game/Ross/Blueprints/InAirComponent.OnGround` (`self.InAirComponent`) _grounddetected)
      ;[1 1 1] Fake Gravity
      (if _grounddetected
        (`self.TestingGravity`)
        ;[0.1289 1 0] Wwise Ground State
        (`AkGameplayStatics.SetState` null "IsOnGround" "OffGround")
        ;[1 1 1] Landing FOV Changes
        (set `self.AirTimer` 1.0)
        (if (> (`self.LandingTimer`) 0.0)
          (if _isboosting
            _
            (elif (not _isovercharging)
              (set `/Game/Micheal/Blueprints/AccelerationComponent.Max FOV` 90.0 _accelerationcomponent)
              (set `/Game/Micheal/Blueprints/AccelerationComponent.Lerp Speed` 2.0 _accelerationcomponent)))
          (elif _isboosting
            _
            (elif (not _isovercharging)
              (set `/Game/Micheal/Blueprints/AccelerationComponent.Max FOV` 120.0 _accelerationcomponent)
              (set `/Game/Micheal/Blueprints/AccelerationComponent.Lerp Speed` 0.5 _accelerationcomponent))))
        (else
          (`PrimitiveComponent.AddForce` (`self.Cube`) (* (`KismetMathLibrary.GetUpVector` (struct)) -1.0 3000.0) "None" true)
          (`AkGameplayStatics.SetState` null "IsOnGround" "OnGround")
          (if (<= (`self.AirTimer`) 0.0)
            (set `self.LandingTimer` 0.5)))))
    (:`then_1`
      ;[1 1 1] Rotation Lerp
      (`SceneComponent.K2_SetRelativeRotation` (`self.boardMesh`) (`KismetMathLibrary.MakeRotator` _returnvalue_roll_2 _returnvalue_pitch _relativerotation_yaw) false false))
    (:`then_2`
      ;[1 0 0] Allows Restarting
      (`KismetSystemLibrary.Delay` 5.0)
      (set `self.CanRestart` true))
    (:`then_3`
      ;[1 0 0] Respawns Player if fall off the map
      (if (< _returnvalue_z 15000.0)
        (`self.K2_DestroyActor`)))
    (:`then_4`
      ;[1 1 1] Lava Check
      (`self.LavaCheck`)
      (`self.DEBUG printTest`))
    (:`then_5`
      ;[1 1 1] Update Timer + Angle Correction
      (`self.UpdateTimer`)
      (`self.AngleCorrection` (`self.Delta Seconds`)))
    (:`then_6`
      ;[0.02316 1 0] Wwise Swoosh Tracer
      (`KismetSystemLibrary.Delay` (`KismetMathLibrary.RandomFloatInRange` 0.1 0.5))
      (`self.NearMissCheck`))))

(event `self.ReceiveDestroyed`
  ;[1 0.01038 0] If player destroyed, respawn
  (`/Game/Ross/Blueprints/CheckpointSystem/CheckpointPlayerController.RespawnVehicle` (`self.CheckpointControllerReference`)))

(event `InputAction|Restart`
  (params (Key :type "Key Structure"))
  ;[1 0 0] Restart level
  (:`Pressed`
    (`KismetSystemLibrary.Delay` 5.0)
    (`KismetSystemLibrary.ExecuteConsoleCommand` "RestartLevel" null)))

(event `InputAction|Death`
  (params (Key :type "Key Structure"))
  ;[1 0 0] Respawn Button 'Z'
  (:`Pressed`
    (if (`self.CanRestart`)
      (`self.K2_DestroyActor`)
      (set `self.CanRestart` false))))

(event `self.Cube.OnComponentBeginOverlap`
  (params (OverlappedComponent :type "PrimitiveComponent Object Reference") (OtherActor :type "Actor Object Reference") (OtherComp :type "PrimitiveComponent Object Reference") (OtherBodyIndex :type Integer) (bFromSweep :type Boolean) (SweepResult :type "HitResult Structure (by ref)"))
  (bind _accelerationcomponent (`self.AccelerationComponent`))
  (bind _accelerationcomponent_2 (`self.AccelerationComponent`))
  ;[1 1 1] Hitting Obstacle
  (`|ExecutionSequence`
    (:`then_0`
      ;[0.25 0.25 0.25] Boost Pickups
      ;;[0 0 0] Boost Pickup (overcharge)
      (if (`self.ActorHasTag` OtherActor "Overcharge")
        (`self.StartOverchargingFOV`)
        (`self.SetActorHiddenInGame` OtherActor true)
        (`self.SetActorEnableCollision` OtherActor false)
        (if (`self.isBoosting`)
          (`|ExecutionSequence`
            (:`then_0`
              (set `/Game/Micheal/Blueprints/AccelerationComponent.Max Acceleration` 7500.0 (`self.AccelerationComponent`))
              (`KismetSystemLibrary.Delay` 3.0)
              (`self.StopBoosting`)
              (`self.EndOverchargingFOV`))
            (:`then_1`
              (`KismetSystemLibrary.Delay` 2.5 :!label _label)
              (`self.SetActorHiddenInGame` OtherActor false)
              (`self.SetActorEnableCollision` OtherActor true)))
          (else
            (set `/Game/Micheal/Blueprints/AccelerationComponent.Max Acceleration` 5000.0 _accelerationcomponent_2)
            (`KismetSystemLibrary.Delay` 3.0)
            (set `/Game/Micheal/Blueprints/AccelerationComponent.Max Acceleration` 3500.0 _accelerationcomponent_2)
            (`self.EndOverchargingFOV`)
            (goto _label)))))
    (:`then_1`
      ;;[0 0 0] Boost Pickup (recharge)
      (if (`self.ActorHasTag` OtherActor "Recharge")
        (`self.SetActorHiddenInGame` OtherActor true)
        (`self.SetActorEnableCollision` OtherActor false)
        (set `self.Boost` (`KismetMathLibrary.Clamp` (+ (`self.Boost`) 66) 0 (`self.MaxBoost`)))
        (`KismetSystemLibrary.Delay` 2.5)
        (`self.SetActorHiddenInGame` OtherActor false)
        (`self.SetActorEnableCollision` OtherActor true)))
    (:`then_2`
      ;;[0 0 0] Boost Pickup (ultimate)
      (if (`self.ActorHasTag` OtherActor "Ultimate")
        (`self.SetActorHiddenInGame` OtherActor true)
        (`self.SetActorEnableCollision` OtherActor false)
        (set `self.Boost` (`KismetMathLibrary.Clamp` (+ (`self.Boost`) 66) 0 (`self.MaxBoost`)))
        (set `/Game/Micheal/Blueprints/AccelerationComponent.Max Acceleration` 4000.0 _accelerationcomponent)
        (`KismetSystemLibrary.Delay` 3.0)
        (set `/Game/Micheal/Blueprints/AccelerationComponent.Max Acceleration` 3500.0 _accelerationcomponent)
        (`KismetSystemLibrary.Delay` 2.5)
        (`self.SetActorHiddenInGame` OtherActor false)
        (`self.SetActorEnableCollision` OtherActor true)))
    (:`then_3`
      (if (`self.ActorHasTag` OtherActor "Obstacle")
        (set `/Game/Micheal/Blueprints/AccelerationComponent.Touching Obstacle` true (`self.AccelerationComponent`))
        (set `/Game/Micheal/Blueprints/AccelerationComponent.Acceleration` 3000.0 (`self.AccelerationComponent`))
        (`KismetSystemLibrary.Delay` 0.25)
        (set `/Game/Micheal/Blueprints/AccelerationComponent.Acceleration` 2000.0 (`self.AccelerationComponent`))))))

(event `self.PlayerModel.OnComponentBeginOverlap`
  (params (OverlappedComponent :type "PrimitiveComponent Object Reference") (OtherActor :type "Actor Object Reference") (OtherComp :type "PrimitiveComponent Object Reference") (OtherBodyIndex :type Integer) (bFromSweep :type Boolean) (SweepResult :type "HitResult Structure (by ref)"))
  ;[1 1 1] Respawn
  (if (`self.ActorHasTag` OtherActor "Ground")
    (set `self.TouchingPlayer` true)
    (`KismetSystemLibrary.Delay` 3.0)
    (if (`/Game/A_ProgrammerCommon/Blueprints/HoverComponent.DetectGround` (`self.UpComponent`))
      (`KismetSystemLibrary.ExecuteConsoleCommand` "RestartLevel" null))))

(event `InputAction|Boost`
  (params (Key :type "Key Structure"))
  ;[0.01181 1 0] Wwise Boost sound
  (:`Pressed`
    (if (`self.isBoosting`)
      (`AkGameplayStatics.PostEvent` "/Game/Dex/Events/PSFX/Boost.Boost" self)
      (set `self.BoostEnded` false)))
  (:`Released`
    (if (not (`self.BoostEnded`))
      (`AkGameplayStatics.PostEvent` "/Game/Dex/Events/PSFX/BoostEnd.BoostEnd" self)
      (set `self.BoostEnded` true))))

(event `InputAction|Boost`
  (params (Key :type "Key Structure"))
  ;[0 0 0] Boost
  (:`Pressed`
    (`self.StartBoosting`))
  (:`Released`
    (`self.StopBoosting`)))

(event `Drain Boost`
  ;[0 0 0] Boost
)

(event `Regen Boost`
  ;[0 0 0] Boost
  (bind _output_get (set `self.Boost` (`KismetMathLibrary.Clamp` (+ (`self.Boost`) 1) 0 (`self.MaxBoost`))))
  (if (== _output_get (`self.MaxBoost`))
    _
    (elif (not (`self.isBoosting`))
      (`KismetSystemLibrary.Delay` 1.5)
      (`self.Regen Boost`))))

(fn `Accelerate`
  (locals (AirVector :type "Vector Structure"))
  (bind _returnvalue (* (`/Game/Micheal/Blueprints/AccelerationComponent.Acceleration` (`self.AccelerationComponent`)) (`SceneComponent.GetForwardVector` (`self.Cube`))))
  (bind _grounddetected (`self.GroundCheck`))
  (if _grounddetected
    ;[0.3228 1 0.31] Does not apply Z axis acceleration if in air
    (`PrimitiveComponent.AddForce` (`self.Cube`) _returnvalue "None" true)
    (else
      (bind _output_get (set `local.AirVector` _returnvalue))
      (`PrimitiveComponent.AddForce` (`self.Cube`) (`KismetMathLibrary.MakeVector` (.x _output_get) (.y _output_get)) "None" true))))

(fn `AngleCorrection`
  (params (DeltaTime :type "Float (double-precision)"))
  (bind (_returnvalue_roll _returnvalue_pitch _returnvalue_yaw) (`KismetMathLibrary.BreakRotator` (`SceneComponent.K2_GetComponentRotation` (`self.Cube`))))
  (bind (_returnvalue_roll_2 _returnvalue_pitch_2 _returnvalue_yaw_2) (`KismetMathLibrary.BreakRotator` (`SceneComponent.K2_GetComponentRotation` (`self.Cube`))))
  (bind (_returnvalue_roll_3 _returnvalue_pitch_3 _returnvalue_yaw_3) (`KismetMathLibrary.BreakRotator` (`SceneComponent.K2_GetComponentRotation` (`self.Cube`))))
  (bind _returnvalue_roll_4 (`KismetMathLibrary.BreakRotator` (`SceneComponent.K2_GetComponentRotation` (`self.Cube`))))
  (`|ExecutionSequence`
    (:`then_0`
      (bind _grounddetected (`self.GroundCheck`))
      (if (not _grounddetected)
        (`SceneComponent.K2_SetRelativeRotation` (`self.Cube`) (`KismetMathLibrary.RInterpTo` (`SceneComponent.K2_GetComponentRotation` (`self.Cube`)) (`KismetMathLibrary.MakeRotator` 0.0 0.0 _returnvalue_yaw_2) DeltaTime 1.0) false false)))
    (:`then_1`
      (if (> _returnvalue_roll_4 60.0)
        (`SceneComponent.K2_SetWorldRotation` (`self.Cube`) (`KismetMathLibrary.MakeRotator` 60.0 _returnvalue_pitch_3 _returnvalue_yaw_3) false false)
        (elif (< _returnvalue_roll_4 -60.0)
          (`SceneComponent.K2_SetWorldRotation` (`self.Cube`) (`KismetMathLibrary.MakeRotator` -60.0 _returnvalue_pitch _returnvalue_yaw) false false))))))

(fn `DEBUG printTest`
  (`KismetSystemLibrary.PrintString` (`KismetStringLibrary.Conv_DoubleToString` (`/Game/Micheal/Blueprints/AccelerationComponent.Lerp Speed` (`self.AccelerationComponent`))))
  (`KismetSystemLibrary.PrintString` (`KismetStringLibrary.Conv_DoubleToString` (`/Game/Micheal/Blueprints/AccelerationComponent.Max FOV` (`self.AccelerationComponent`)))))

(fn `EndOverchargingFOV`
  (set `/Game/Micheal/Blueprints/AccelerationComponent.Lerp Speed` 0.5 (`self.AccelerationComponent`))
  (set `/Game/Micheal/Blueprints/AccelerationComponent.Max FOV` 120.0 (`self.AccelerationComponent`))
  (set `self.isOvercharging` false))

(fn `GroundCheck`
  (returns (GroundDetected :type Boolean))
  (return (or (`/Game/A_ProgrammerCommon/Blueprints/HoverComponent.DetectGround` (`self.HoverComponent`)) (`/Game/A_ProgrammerCommon/Blueprints/HoverComponent.DetectGround` (`self.HoverComponent1`)) (`/Game/A_ProgrammerCommon/Blueprints/HoverComponent.DetectGround` (`self.HoverComponent2`)) (`/Game/A_ProgrammerCommon/Blueprints/HoverComponent.DetectGround` (`self.HoverComponent3`)))))

(fn `LavaCheck`
  (bind _accelerationcomponent (`self.AccelerationComponent`))
  (bind _accelerationcomponent_2 (`self.AccelerationComponent`))
  (bind _accelerationcomponent_3 (`self.AccelerationComponent`))
  (if (or (`/Game/A_ProgrammerCommon/Blueprints/HoverComponent.Touching Lava` (`self.HoverComponent3`)) (`/Game/A_ProgrammerCommon/Blueprints/HoverComponent.Touching Lava` (`self.HoverComponent2`)) (`/Game/A_ProgrammerCommon/Blueprints/HoverComponent.Touching Lava` (`self.HoverComponent1`)) (`/Game/A_ProgrammerCommon/Blueprints/HoverComponent.Touching Lava` (`self.HoverComponent`)))
    (set `/Game/Micheal/Blueprints/AccelerationComponent.TempMaxAccel` 2500.0 _accelerationcomponent_2)
    (set `/Game/Micheal/Blueprints/AccelerationComponent.Aimed FOV` 60.0 _accelerationcomponent_2)
    (set `/Game/Micheal/Blueprints/AccelerationComponent.Lerp Speed` 1.75 _accelerationcomponent_2)
    ;[0 1 0.009654] Wwise Lava State
    (`AkGameplayStatics.SetState` null "IsOnLava" "OnLava")
    (elif (> (`/Game/Micheal/Blueprints/AccelerationComponent.Max Acceleration` _accelerationcomponent) (`/Game/Micheal/Blueprints/AccelerationComponent.TempMaxAccel` _accelerationcomponent))
      (set `/Game/Micheal/Blueprints/AccelerationComponent.TempMaxAccel` (`/Game/Micheal/Blueprints/AccelerationComponent.Max Acceleration` _accelerationcomponent_3) _accelerationcomponent_3)
      (if (`self.isOvercharging`)
        (set `/Game/Micheal/Blueprints/AccelerationComponent.Lerp Speed` 2.0 _accelerationcomponent_3)
        (else
          (set `/Game/Micheal/Blueprints/AccelerationComponent.Lerp Speed` 0.5 _accelerationcomponent_3)))
      (`AkGameplayStatics.SetState` null "IsOnLava" "OffLava"))))

(fn `NearMissCheck`
  (bind _returnvalue (`SceneComponent.K2_GetComponentLocation` (`self.boardMesh`)))
  (bind (_outhit _returnvalue_2) (`KismetSystemLibrary.SphereTraceSingle` :`Start` _returnvalue :`End` _returnvalue :`Radius` 300.0 :`TraceChannel` "TraceTypeQuery4" :`bTraceComplex` true :`DrawDebugType` "ForOneFrame"))
  (if _returnvalue_2
    (`AkGameplayStatics.PostEvent` "/Game/Dex/Events/LSFX/Swoosh.Swoosh" self)))

(fn `RespawnCheck`
  (returns (IsPlayerStuck :type Boolean))
  (if (`/Game/A_ProgrammerCommon/Blueprints/HoverComponent.DetectGround` (`self.UpComponent`))
    (set `self.IsStuck` true)
    (else
      (set `self.IsStuck` false)))
  (return (`self.IsStuck`)))

(fn `StartBoosting`
  (set `/Game/Micheal/Blueprints/AccelerationComponent.Max Acceleration` 5000.0 (`self.AccelerationComponent`))
  (set `self.isBoosting` true)
  (`self.Drain Boost`)
  (if (`self.isOvercharging`)
    (set `/Game/Micheal/Blueprints/AccelerationComponent.Max FOV` 160.0 (`self.AccelerationComponent`))
    (else
      (set `/Game/Micheal/Blueprints/AccelerationComponent.Max FOV` 145.0 (`self.AccelerationComponent`)))))

(fn `StartOverchargingFOV`
  (set `self.isOvercharging` true)
  (set `/Game/Micheal/Blueprints/AccelerationComponent.Lerp Speed` 2.0 (`self.AccelerationComponent`))
  (if (`self.isBoosting`)
    (set `/Game/Micheal/Blueprints/AccelerationComponent.Max FOV` 160.0 (`self.AccelerationComponent`))
    (else
      (set `/Game/Micheal/Blueprints/AccelerationComponent.Max FOV` 145.0 (`self.AccelerationComponent`)))))

(fn `StopBoosting`
  (bind _accelerationcomponent (`self.AccelerationComponent`))
  (set `/Game/Micheal/Blueprints/AccelerationComponent.Max Acceleration` 3500.0 _accelerationcomponent)
  (set `/Game/Micheal/Blueprints/AccelerationComponent.Max FOV` 120.0 _accelerationcomponent)
  (if (`self.isOvercharging`)
    (set `/Game/Micheal/Blueprints/AccelerationComponent.Lerp Speed` 2.0 _accelerationcomponent)
    (else
      (set `/Game/Micheal/Blueprints/AccelerationComponent.Lerp Speed` 0.5 _accelerationcomponent)))
  (set `self.isBoosting` false)
  (`self.Regen Boost`))

(fn `TestingGravity`
  (for _array_element (`self.HoverComponentArray`)
    (if (`/Game/A_ProgrammerCommon/Blueprints/HoverComponent.DetectGround` _array_element)
      (set `self.GravityDirection` (+ (`/Game/A_ProgrammerCommon/Blueprints/HoverComponent.Impact Normal` _array_element) (`self.GravityDirection`)))
      (`/Engine/EditorBlueprintResources/StandardMacros.IncrementInt` (`self.NormalsNum`))))
  (`PrimitiveComponent.AddForce` (`self.Cube`) (* (/ (`self.GravityDirection`) (`self.NormalsNum`)) -1.0 2000.0) "None" true)
  (set `self.GravityDirection` (0.0 0.0 0.0))
  (set `self.NormalsNum` 0))

(fn `UpdateTimer`
  (bind _grounddetected (`self.GroundCheck`))
  (if _grounddetected
    (if (> (`self.LandingTimer`) 0.0)
      (set `self.LandingTimer` (- (`self.LandingTimer`) (`self.Delta Seconds`))))
    (elif (> (`self.AirTimer`) 0.0)
      (set `self.AirTimer` (- (`self.AirTimer`) (`self.Delta Seconds`))))))

(fn `UserConstructionScript`)

(fn `WwiseSetup`
  (`PlayerController.SetAudioListenerOverride` :`self` (`GameplayStatics.GetPlayerController` 0) :`AttachToComponent` (`self.Cube`))
  (`AkGameplayStatics.PostEvent` "/Game/Dex/Events/MM/PlayFoundry.PlayFoundry" self)
  (`AkGameplayStatics.PostEvent` "/Game/Dex/Events/PSFX/HoverIdle.HoverIdle" self)
  (`AkGameplayStatics.PostEvent` "/Game/Dex/Events/PSFX/HoverForward.HoverForward" self)
  (`AkGameplayStatics.SetState` null "IsOnLava" "OffLava")
  (`AkGameplayStatics.SetState` null "IsOnGround" "OnGround"))