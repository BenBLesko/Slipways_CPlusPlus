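; Hover component that keeps the player's physics-simulated mesh floating above surfaces tagged Ground.
; InitComponent stores the mesh and enables physics on it.
; Each tick a debug-drawn trace runs down the component's local up axis, updating ground and lava-material flags.
; On tagged hits it applies force along the surface normal at its own location, fading with distance like a spring, and sets linear and angular damping.
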(event `InitComponent`
  (params (MeshComponent :type "StaticMeshComponent Object Reference"))
  ;[1 1 1] Simulates Physics for the Player
  (bind _output_get (set `self.ParentComponent` MeshComponent))
  (`PrimitiveComponent.SetSimulatePhysics` _output_get true))

(event `self.ReceiveTick`
  (params (DeltaSeconds :type "Float (single-precision)"))
  (bind _returnvalue (`self.K2_GetComponentLocation`))
  (bind (_outhit _returnvalue_2) (`KismetSystemLibrary.LineTraceSingle` :`Start` _returnvalue :`End` (+ _returnvalue (* (`self.GetUpVector`) (* (`self.traceLength`) -1.0))) :`TraceChannel` "TraceTypeQuery3" :`DrawDebugType` "ForDuration" :`DrawTime` 0.01))
  (bind (_bblockinghit _binitialoverlap _time _distance _location _impactpoint _normal _impactnormal _physmat _hitactor) (`GameplayStatics.BreakHitResult` _outhit))
  (set `self.Touching Lava` (== (`self.Lava Physics Material`) _physmat))
  ;[1 1 1] Continues if raycast hits the ground
  (bind _output_get (set `self.DetectGround` _returnvalue_2))
  (if _output_get
    (if (`Actor.ActorHasTag` _hitactor "Ground")
      (`PrimitiveComponent.AddForceAtLocation` (`self.ParentComponent`) (* _impactnormal (`KismetMathLibrary.Lerp` (`self.HoverForce`) 0.0 (/ (`KismetMathLibrary.VSize` (- _location (`self.K2_GetComponentLocation`))) (`self.traceLength`)))) (`self.K2_GetComponentLocation`) "None")
      (`PrimitiveComponent.SetLinearDamping` (`self.ParentComponent`) 1.0) ; Careful, Don't increase above ~0.8f
      (`PrimitiveComponent.SetAngularDamping` (`self.ParentComponent`) 7.0))))