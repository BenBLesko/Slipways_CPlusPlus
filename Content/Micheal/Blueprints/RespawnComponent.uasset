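; RespawnComponent is a component meant to return a cube to a spawn point when the player presses R.
; Its unconnected logic polls the R key, then moves the cube to the SpawnPoint actor, zeroes the acceleration component's Acceleration and resets rotation.
; InitComponent and Tick are empty, and both the reference assignments and the respawn chain are disconnected, so the component currently does nothing.
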(event `Init Component`
  (params (Cube :type "StaticMeshComponent Object Reference") (`Acc. Comp.` :type "/Game/Micheal/Blueprints/AccelerationComponent Object Reference")))

(event `self.ReceiveTick`
  (params (DeltaSeconds :type "Float (single-precision)")))