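; Spline-driven slipway builder that generates a track section or scatters obstacles in the construction script, switched by IsSlip.
; Slip mode derives offset wall splines (left reversed), lays spline meshes for track and optional walls, and adds instanced pillars and randomly jittered girders.
; Obstacle mode picks random vat, ramp and crucible meshes along a vertically offset spline, line-traces downward, and sinks them along the hit normal with random rotation.
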(fn `UserConstructionScript`
  (locals (`Spline Pos` :type "Array of Vector Structure"))
  (bind _returnvalue_x (`KismetMathLibrary.BreakVector` (`self.GetActorScale3D`)))
  (bind _r_wall_spline_pos (`self.R Wall Spline Pos`))
  (bind _trackside (`self.Trackside`))
  (bind _horizontal_random (`self.Horizontal Random`))
  (bind _l_wall_spline_pos (`self.L Wall Spline Pos`))
  (bind _slip_length (`self.Slip Length`))
  (bind _spline (`self.Spline`))
  (bind _instance_pillar (`self.Instance Pillar`))
  (bind _spline_pos (`local.Spline Pos`))
  (bind _spline_wall_r (`self.Spline Wall R`))
  (bind _instance_pillar_2 (`self.Instance Pillar`))
  (bind _spline_wall_l (`self.Spline Wall L`))
  (bind _slip_length_2 (`self.Slip Length`))
  (bind _slip_length_3 (`self.Slip Length`))
  (bind _spline_2 (`self.Spline`))
  (bind _girder_horizontal_offset_random_max (`self.Girder Horizontal Offset Random Max`))
  (bind _girder_rotation_xy_random_max (`self.Girder Rotation XY Random Max`))
  (bind _girder_rotation_z_random_max (`self.Girder Rotation Z Random Max`))
  (bind _obstacle_spline (`self.Obstacle Spline`))
  (bind _xy_rotation_max (`self.XY Rotation Max`))
  (bind _obstaclearray (`self.ObstacleArray`))
  (bind _spline_3 (`self.Spline`))
  (bind _returnvalue (`SplineComponent.GetNumberOfSplinePoints` _spline_3))
  (bind _returnvalue_2 (* -1.0 _xy_rotation_max))
  (bind _returnvalue_3 (* -1.0 _girder_horizontal_offset_random_max))
  (bind _returnvalue_4 (* -1.0 _girder_rotation_xy_random_max))
  (bind (_min _max) (break `Box` (`StaticMesh.GetBoundingBox` (`self.Girder`))))
  (bind _returnvalue_5 (`KismetMathLibrary.RandomFloatInRange` (* -1.0 _horizontal_random) _horizontal_random))
  (if (`self.IsSlip`)
    ;[1 1 1] Instance Adding
    (`StaticMeshComponent.SetStaticMesh` (`self.Instance Pillar`) (`self.Pillar`))
    (`StaticMeshComponent.SetStaticMesh` (`self.Instance Beam`) (`self.Girder`))
    ;[1 1 1] Spline Generation
    (bind _returnvalue_6 (`AddComponent|NODE_AddSplineComponent-0`))
    (bind _output_get (set `self.Spline Wall R` _returnvalue_6))
    (bind _returnvalue_7 (`AddComponent|NODE_AddSplineComponent-1`))
    (bind _output_get_2 (set `self.Spline Wall L` _returnvalue_7))
    (for _index (range (+ _returnvalue 1))
      (bind _returnvalue_8 (- (- _returnvalue 1) _index))
      (bind _returnvalue_9 (`SplineComponent.GetLocationAtSplinePoint` _spline_3 _returnvalue_8 "Local"))
      ;;[1 1 1] Left Side
      (`KismetArrayLibrary.Array_Add` _l_wall_spline_pos (`KismetMathLibrary.MakeVector` (.x (+ (* (* (`KismetMathLibrary.GetRightVector` (`SplineComponent.GetRotationAtSplinePoint` _spline_3 _returnvalue_8 "Local")) (-1.0 -1.0 0.0)) (`self.Walls Offset`)) _returnvalue_9)) (.y (+ (* (* (`KismetMathLibrary.GetRightVector` (`SplineComponent.GetRotationAtSplinePoint` _spline_3 _returnvalue_8 "Local")) (-1.0 -1.0 0.0)) (`self.Walls Offset`)) _returnvalue_9)) (+ (.z _returnvalue_9) (`self.Walls Vertical Offset`))))
      (bind _returnvalue_10 (`SplineComponent.GetLocationAtSplinePoint` _spline_3 _index "Local"))
      ;;[1 1 1] Right Side
      (`KismetArrayLibrary.Array_Add` _r_wall_spline_pos (`KismetMathLibrary.MakeVector` (.x (+ (* (`KismetMathLibrary.GetRightVector` (`SplineComponent.GetRotationAtSplinePoint` _spline_3 _index "Local")) (`self.Walls Offset`)) _returnvalue_10)) (.y (+ (* (`KismetMathLibrary.GetRightVector` (`SplineComponent.GetRotationAtSplinePoint` _spline_3 _index "Local")) (`self.Walls Offset`)) _returnvalue_10)) (+ (.z _returnvalue_10) (`self.Walls Vertical Offset`)))))
    (`SplineComponent.SetSplinePoints` _output_get_2 _l_wall_spline_pos "Local" true)
    (`SplineComponent.SetSplinePoints` _output_get _r_wall_spline_pos "Local" true)
    (for _index_2 (range (+ (`KismetMathLibrary.FTrunc` (/ (`SplineComponent.GetSplineLength` (`self.Spline`)) (`self.Slip Length`))) 1))
      (`|ExecutionSequence`
        (:`then_0`
          ;[1 1 1] Trackside L
          (if (`self.IsWallLOn`)
            (bind _returnvalue_11 (`AddComponent|NODE_AddSplineMeshComponent-2`))
            (`StaticMeshComponent.SetStaticMesh` _returnvalue_11 _trackside)
            (bind _returnvalue_12 (* _slip_length_2 _index_2))
            (bind _returnvalue_13 (* _slip_length_2 (+ _index_2 1)))
            (`SplineMeshComponent.SetStartAndEnd` _returnvalue_11 (`SplineComponent.GetLocationAtDistanceAlongSpline` _spline_wall_l _returnvalue_12 "Local") (`SplineComponent.GetTangentAtDistanceAlongSpline` _spline_wall_l _returnvalue_12 "Local") (`SplineComponent.GetLocationAtDistanceAlongSpline` _spline_wall_l _returnvalue_13 "Local") (`SplineComponent.GetTangentAtDistanceAlongSpline` _spline_wall_l _returnvalue_13 "Local") true)
            (`SceneComponent.K2_AttachToComponent` _returnvalue_11 (`self.DefaultSceneRoot`) "None" "KeepRelative" "KeepRelative" "KeepRelative" true)))
        (:`then_1`
          ;[1 1 1] Trackside R
          (if (`self.IsWallROn`)
            (bind _returnvalue_14 (`AddComponent|NODE_AddSplineMeshComponent-1`))
            (`StaticMeshComponent.SetStaticMesh` _returnvalue_14 _trackside)
            (bind _returnvalue_15 (* _index_2 _slip_length))
            (bind _returnvalue_16 (* _slip_length (+ _index_2 1)))
            (`SplineMeshComponent.SetStartAndEnd` _returnvalue_14 (`SplineComponent.GetLocationAtDistanceAlongSpline` _spline_wall_r _returnvalue_15 "Local") (`SplineComponent.GetTangentAtDistanceAlongSpline` _spline_wall_r _returnvalue_15 "Local") (`SplineComponent.GetLocationAtDistanceAlongSpline` _spline_wall_r _returnvalue_16 "Local") (`SplineComponent.GetTangentAtDistanceAlongSpline` _spline_wall_r _returnvalue_16 "Local") true)
            (`SceneComponent.K2_AttachToComponent` _returnvalue_14 (`self.DefaultSceneRoot`) "None" "KeepRelative" "KeepRelative" "KeepRelative" true)))
        (:`then_2`
          ;[1 1 1] Track
          (bind _returnvalue_17 (`AddComponent|NODE_AddSplineMeshComponent-0`))
          (`StaticMeshComponent.SetStaticMesh` _returnvalue_17 (`self.splineMesh`))
          (`PrimitiveComponent.SetCollisionEnabled` _returnvalue_17 "QueryAndPhysics")
          (bind _returnvalue_18 (* _slip_length_3 _index_2))
          (bind _returnvalue_19 (* _slip_length_3 (+ _index_2 1)))
          (`SplineMeshComponent.SetStartAndEnd` _returnvalue_17 (`SplineComponent.GetLocationAtDistanceAlongSpline` _spline _returnvalue_18 "Local") (`SplineComponent.GetTangentAtDistanceAlongSpline` _spline _returnvalue_18 "Local") (`SplineComponent.GetLocationAtDistanceAlongSpline` _spline _returnvalue_19 "Local") (`KismetMathLibrary.ClampVectorSize` (`SplineComponent.GetTangentAtDistanceAlongSpline` _spline _returnvalue_19 "Local") 0.0 (`self.Slip Length`)) true)
          (`SceneComponent.K2_AttachToComponent` _returnvalue_17 (`self.DefaultSceneRoot`) "None" "KeepRelative" "KeepRelative" "KeepRelative" true))
        (:`then_3`
          ;[1 1 1] Pillars
          ;;[1 1 1] L Base
          (if (`self.IsWallLOn`) :!label _label
            (bind _location (.location (`SplineComponent.GetTransformAtDistanceAlongSpline` (`self.Spline Wall L`) (* (`self.Slip Length`) _index_2) "Local" false)))
            (bind _rotation (.rotation (`SplineComponent.GetTransformAtDistanceAlongSpline` (`self.Spline Wall L`) (* (`self.Slip Length`) _index_2) "Local" false)))
            (`InstancedStaticMeshComponent.AddInstance` _instance_pillar_2 (`KismetMathLibrary.MakeTransform` (`KismetMathLibrary.MakeVector` (.x (+ (* (`KismetMathLibrary.GetRightVector` _rotation) (* (`self.Pillars Offset`) -1.0)) _location)) (.y (+ (* (`KismetMathLibrary.GetRightVector` _rotation) (* (`self.Pillars Offset`) -1.0)) _location)) (+ (.z _location) (`self.Pillar Vertical Offset`))) _rotation) false)
            (`PrimitiveComponent.SetCollisionEnabled` _instance_pillar_2 "QueryAndPhysics")))
        (:`then_4`
          (if (`self.IsWallROn`) :!label _label_2
            (bind _location_2 (.location (`SplineComponent.GetTransformAtDistanceAlongSpline` (`self.Spline Wall R`) (* (`self.Slip Length`) _index_2) "Local" false)))
            (bind _rotation_2 (.rotation (`SplineComponent.GetTransformAtDistanceAlongSpline` (`self.Spline Wall R`) (* (`self.Slip Length`) _index_2) "Local" false)))
            ;;[1 1 1] R Base
            (`InstancedStaticMeshComponent.AddInstance` _instance_pillar (`KismetMathLibrary.MakeTransform` (`KismetMathLibrary.MakeVector` (.x (+ (* (`KismetMathLibrary.GetRightVector` _rotation_2) (* (`self.Pillars Offset`) -1.0)) _location_2)) (.y (+ (* (`KismetMathLibrary.GetRightVector` _rotation_2) (* (`self.Pillars Offset`) -1.0)) _location_2)) (+ (.z _location_2) (`self.Pillar Vertical Offset`))) _rotation_2) false)
            (`PrimitiveComponent.SetCollisionEnabled` _instance_pillar "QueryAndPhysics")))))
    (`|ExecutionSequence`
      (:`then_0`
        (goto _label))
      (:`then_1`
        (goto _label_2))
      (:`then_2`
        ;[1 1 1] Top Girders
        ;;[1 1 1] Get Asset Size and set up mesh
        (if (`self.IaGirderOn`)
          (bind _output_get_3 (set `self.Girder Section Length Coeff` (+ (- (.x _max) (.x _min)) (`self.Girder Horizontal Offset`))))
          ;;[1 1 1] Section length = mesh Length
          (set `self.Girder Section Length` (* _returnvalue_x _output_get_3))
          (for _index_3 (range (`KismetMathLibrary.FTrunc` (/ (`SplineComponent.GetSplineLength` (`self.Spline`)) (`self.Girder Section Length`))))
            (bind _returnvalue_20 (* _index_3 (`self.Girder Section Length`)))
            (bind _returnvalue_21 (`SplineComponent.GetRotationAtDistanceAlongSpline` _spline_2 _returnvalue_20 "Local"))
            (bind (_x _y _z) (`KismetMathLibrary.BreakVector3f` (`SplineComponent.GetLocationAtDistanceAlongSpline` _spline_2 _returnvalue_20 "Local")))
            (`InstancedStaticMeshComponent.AddInstance` (`self.Instance Beam`) (`KismetMathLibrary.MakeTransform` (`KismetMathLibrary.MakeVector` (+ (.x (* (`KismetMathLibrary.GetForwardVector` _returnvalue_21) (`KismetMathLibrary.MakeVector` (`KismetMathLibrary.RandomFloatInRange` _returnvalue_3 _girder_horizontal_offset_random_max) (`KismetMathLibrary.RandomFloatInRange` _returnvalue_3 _girder_horizontal_offset_random_max)))) _x) (+ (.y (* (`KismetMathLibrary.GetForwardVector` _returnvalue_21) (`KismetMathLibrary.MakeVector` (`KismetMathLibrary.RandomFloatInRange` _returnvalue_3 _girder_horizontal_offset_random_max) (`KismetMathLibrary.RandomFloatInRange` _returnvalue_3 _girder_horizontal_offset_random_max)))) _y) (+ _z (`self.Girder Vertical Offset`) 0.0)) (`KismetMathLibrary.MakeRotator` (+ (`KismetMathLibrary.RandomFloatInRange` _returnvalue_4 _girder_rotation_xy_random_max) (.roll _returnvalue_21)) (+ (`KismetMathLibrary.RandomFloatInRange` _returnvalue_4 _girder_rotation_xy_random_max) (.pitch _returnvalue_21)) (+ (`KismetMathLibrary.RandomFloatInRange` (* -1.0 _girder_rotation_z_random_max) _girder_rotation_z_random_max) (.yaw _returnvalue_21)))) false)))))
    (else
      ;[1 1 1] Array Creation
      (`KismetArrayLibrary.Array_Add` _obstaclearray "/Game/A_AssetsFromTony/Models/Obstacle_Flexible_Crucible.Obstacle_Flexible_Crucible")
      (`KismetArrayLibrary.Array_Add` _obstaclearray "/Game/A_AssetsFromTony/Models/Obstacle_Jump_Vat_1.Obstacle_Jump_Vat_1")
      (`KismetArrayLibrary.Array_Add` _obstaclearray "/Game/A_AssetsFromTony/Models/Obstacle_Jump_Vat_2.Obstacle_Jump_Vat_2")
      (`KismetArrayLibrary.Array_Add` _obstaclearray "/Game/A_AssetsFromTony/Models/Obstacle_Jump_Vat_3.Obstacle_Jump_Vat_3")
      (`KismetArrayLibrary.Array_Add` _obstaclearray "/Game/A_AssetsFromTony/Models/Obstacle_Jump_Vat_4.Obstacle_Jump_Vat_4")
      (`KismetArrayLibrary.Array_Add` _obstaclearray "/Game/A_AssetsFromTony/Models/Obstacle_Jump_Vat_5.Obstacle_Jump_Vat_5")
      (`KismetArrayLibrary.Array_Add` _obstaclearray "/Game/A_AssetsFromTony/Models/Obstacle_Ramp_Containers_1.Obstacle_Ramp_Containers_1")
      ;[1 1 1] Spline
      (bind _returnvalue_22 (`AddComponent|NODE_AddSplineComponent-2`))
      (set `self.Obstacle Spline` _returnvalue_22)
      (for _index_4 (range (+ (`SplineComponent.GetNumberOfSplinePoints` (`self.Spline`)) 1))
        (`KismetArrayLibrary.Array_Add` _spline_pos (`KismetMathLibrary.MakeVector` (.x (`SplineComponent.GetLocationAtSplinePoint` (`self.Spline`) _index_4 "Local")) (.y (`SplineComponent.GetLocationAtSplinePoint` (`self.Spline`) _index_4 "Local")) (+ (.z (`SplineComponent.GetLocationAtSplinePoint` (`self.Spline`) _index_4 "Local")) (`self.Vertical Offset`)))))
      (`SplineComponent.SetSplinePoints` (`self.Obstacle Spline`) _spline_pos "Local" true)
      (for _index_5 (range (`KismetMathLibrary.FTrunc` (/ (`SplineComponent.GetSplineLength` (`self.Obstacle Spline`)) (`self.Density`))))
        (set `self.ObstacleChosen` (`KismetArrayLibrary.Array_Random` (`self.ObstacleArray`)))
        (bind _returnvalue_23 (* _index_5 (`self.Density`)))
        (bind _returnvalue_24 (`SplineComponent.GetRotationAtDistanceAlongSpline` _obstacle_spline _returnvalue_23 "World"))
        (bind (_x_2 _y_2 _z_2) (`KismetMathLibrary.BreakVector3f` (`SplineComponent.GetLocationAtDistanceAlongSpline` _obstacle_spline _returnvalue_23 "World")))
        (bind _returnvalue_25 (`KismetMathLibrary.MakeVector` (+ (.x (* (`KismetMathLibrary.GetRightVector` _returnvalue_24) (`KismetMathLibrary.MakeVector` _returnvalue_5 _returnvalue_5))) _x_2) (+ (.y (* (`KismetMathLibrary.GetRightVector` _returnvalue_24) (`KismetMathLibrary.MakeVector` _returnvalue_5 _returnvalue_5))) _y_2) _z_2))
        ;[1 1 1] Line Trace
        (bind _outhit (`KismetSystemLibrary.LineTraceSingle` :`Start` _returnvalue_25 :`End` (+ _returnvalue_25 (* (`KismetMathLibrary.GetUpVector` _returnvalue_24) (* (`self.TraceLength`) -1.0))) :`TraceChannel` "TraceTypeQuery3" :`bTraceComplex` true :`TraceColor` (struct :`R` 1.0 :`B` 0.915275 :`A` 1.0) :`TraceHitColor` (struct :`R` 0.01163 :`B` 1.0 :`A` 1.0) :`DrawTime` 0.01))
        (bind (_bblockinghit _binitialoverlap _time _distance _location_3 _impactpoint _normal) (`GameplayStatics.BreakHitResult` _outhit))
        ;[1 1 1] Add Mesh
        (bind _returnvalue_26 (`AddComponent|NODE_AddStaticMeshComponent-16` :`bManualAttachment` true :`RelativeTransform` (`KismetMathLibrary.MakeTransform` (- _location_3 (* _normal (/ (.z (`.Max` (break `Box` (`StaticMesh.GetBoundingBox` (`self.ObstacleChosen`))))) (`self.Dig in`)))) (`KismetMathLibrary.MakeRotator` (`KismetMathLibrary.RandomFloatInRange` _returnvalue_2 _xy_rotation_max) (`KismetMathLibrary.RandomFloatInRange` _returnvalue_2 _xy_rotation_max) (`KismetMathLibrary.RandomFloatInRange` -360.0 360.0)))))
        (`StaticMeshComponent.SetStaticMesh` _returnvalue_26 (`self.ObstacleChosen`))))))