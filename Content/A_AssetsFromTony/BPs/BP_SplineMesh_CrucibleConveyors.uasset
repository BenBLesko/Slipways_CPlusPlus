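; Spline-driven construction actor that builds a crucible conveyor along an editable spline, with no active runtime logic.
; The construction script stretches a spline mesh between each pair of spline points, with query and physics collision.
; It then places instanced asset and support meshes along the spline at intervals derived from the asset's bounding-box length plus a horizontal offset and actor X scale, lowered by a vertical offset.
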(fn `UserConstructionScript`
  (bind _returnvalue_x (`KismetMathLibrary.BreakVector` (`self.GetActorScale3D`)))
  (bind _asset (`self.Asset`))
  (bind _spline (`self.Spline`))
  (bind _spline_2 (`self.Spline`))
  (bind _spline_3 (`self.Spline`))
  (bind _returnvalue (* (`self.Current Index`) (`self.Section Length`)))
  (bind (_min _max) (break `Box` (`StaticMesh.GetBoundingBox` _asset)))
  (bind (_x _y _z) (`KismetMathLibrary.BreakVector3f` (`SplineComponent.GetLocationAtDistanceAlongSpline` _spline _returnvalue "Local")))
  (bind _returnvalue_2 (`KismetMathLibrary.MakeTransform` (`KismetMathLibrary.MakeVector` _x _y (+ _z (* (`self.Vertical Offset`) -1.0))) (`SplineComponent.GetRotationAtDistanceAlongSpline` _spline _returnvalue "Local")))
  (`|ExecutionSequence`
    (:`then_0`
      ;[1 1 1] Spline Mesh Data
      (for _index (range (+ (- (`SplineComponent.GetNumberOfSplinePoints` (`self.Spline`)) 2) 1))
        ;[1 1 1] Top Part
        (bind _returnvalue_3 (`AddComponent|NODE_AddSplineMeshComponent-0`))
        (`StaticMeshComponent.SetStaticMesh` _returnvalue_3 (`self.splineMesh`))
        (`PrimitiveComponent.SetCollisionEnabled` _returnvalue_3 "QueryAndPhysics")
        (bind _returnvalue_4 (+ _index 1))
        (`SplineMeshComponent.SetStartAndEnd` _returnvalue_3 (`SplineComponent.GetLocationAtSplinePoint` _spline_3 _index "Local") (`SplineComponent.GetTangentAtSplinePoint` _spline_3 _index "Local") (`SplineComponent.GetLocationAtSplinePoint` _spline_2 _returnvalue_4 "Local") (`SplineComponent.GetTangentAtSplinePoint` _spline_2 _returnvalue_4 "Local") true)
        (`SceneComponent.K2_AttachToComponent` _returnvalue_3 (`self.DefaultSceneRoot`) "None" "KeepRelative" "KeepRelative" "KeepRelative" true)))
    (:`then_1`
      ;[1 1 1] Get Asset Size and set up mesh
      (`StaticMeshComponent.SetStaticMesh` (`self.InstancedAsset`) _asset)
      (`StaticMeshComponent.SetStaticMesh` (`self.InstancedConnector`) (`self.Support`))
      (bind _output_get (set `self.Section Length Coeff` (+ (- (.x _max) (.x _min)) (`self.Horizontal Offset`))))
      ;[1 1 1] Section length = mesh Length
      (set `self.Section Length` (* _returnvalue_x _output_get))
      (for _index_2 (range (`KismetMathLibrary.FTrunc` (/ (`SplineComponent.GetSplineLength` (`self.Spline`)) (`self.Section Length`))))
        (set `self.Current Index` _index_2)
        (`InstancedStaticMeshComponent.AddInstance` (`self.InstancedAsset`) _returnvalue_2 false)
        (`InstancedStaticMeshComponent.AddInstance` (`self.InstancedConnector`) _returnvalue_2 false)))))