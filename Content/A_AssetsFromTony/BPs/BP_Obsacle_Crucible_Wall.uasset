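; Crucible wall obstacle that builds a modular support wall and a falling molten stream in its construction script.
; Instanced mesh components repeat the support along negative local Y and the stream downward in world space from the molten top, using configurable lengths.
; Mesh bounding boxes set the spacing, so swapped meshes still tile.
; After the stream loop, an extra segment and a bottom piece are placed at the end.
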(fn `UserConstructionScript`
  (bind (_min _max) (break `Box` (`StaticMesh.GetBoundingBox` (`self.Stream ref`))))
  (bind (_min_2 _max_2) (break `Box` (`StaticMesh.GetBoundingBox` (`self.Wall Supp`))))
  (`StaticMeshComponent.SetStaticMesh` (`self.Support`) (`self.Wall Supp`))
  (`StaticMeshComponent.SetStaticMesh` (`self.Stream`) (`self.Stream ref`))
  (`StaticMeshComponent.SetStaticMesh` (`self.Stream_Bot`) (`self.Stream Bot Ref`))
  (`|ExecutionSequence`
    (:`then_0`
      ;[1 1 1] Get Asset Size and set up mesh
      (bind _output_get (set `self.Section Length Coeff` (- (.y _max_2) (.y _min_2))))
      ;[1 1 1] Placement loop
      (for _index (range (+ (`self.Support lenghth`) 1))
        (`InstancedStaticMeshComponent.AddInstance` (`self.Support`) (`KismetMathLibrary.MakeTransform` (`KismetMathLibrary.MakeVector` (.x (.location (`SceneComponent.GetRelativeTransform` (`self.Obstace_Flexible_Crucible_Wall_support_1`)))) (+ (* (* _output_get _index) -1.0) (.y (.location (`SceneComponent.GetRelativeTransform` (`self.Obstace_Flexible_Crucible_Wall_support_1`))))) (.z (.location (`SceneComponent.GetRelativeTransform` (`self.Obstace_Flexible_Crucible_Wall_support_1`))))) (.rotation (`SceneComponent.GetRelativeTransform` (`self.Obstace_Flexible_Crucible_Wall_support_1`))) (.scale (`SceneComponent.GetRelativeTransform` (`self.Obstace_Flexible_Crucible_Wall_support_1`)))) false)))
    (:`then_1`
      ;[1 1 1] Get Asset Size and set up mesh
      (bind _output_get_2 (set `self.Section Length Coeff lava` (- (.z _max) (.z _min))))
      ;[1 1 1] Placement loop
      (for _index_2 (range (+ (`self.Lava Length`) 1))
        (bind _returnvalue (`KismetMathLibrary.MakeTransform` (`KismetMathLibrary.MakeVector` (.x (.location (`SceneComponent.K2_GetComponentToWorld` (`self.Obstacle_Dodge_Molten__Top`)))) (.y (.location (`SceneComponent.K2_GetComponentToWorld` (`self.Obstacle_Dodge_Molten__Top`)))) (+ (- (* (* _output_get_2 _index_2) -1.0) _output_get_2) (.z (.location (`SceneComponent.K2_GetComponentToWorld` (`self.Obstacle_Dodge_Molten__Top`)))))) (.rotation (`SceneComponent.K2_GetComponentToWorld` (`self.Obstacle_Dodge_Molten__Top`))) (.scale (`SceneComponent.K2_GetComponentToWorld` (`self.Obstacle_Dodge_Molten__Top`)))))
        (`InstancedStaticMeshComponent.AddInstance` (`self.Stream`) _returnvalue true :!label _label))
      (`|ExecutionSequence`
        (:`then_0`
          (goto _label))
        (:`then_1`
          (`InstancedStaticMeshComponent.AddInstance` (`self.Stream_Bot`) _returnvalue true))))))