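; BP_BoostPickUp is a boost pickup actor; this Blueprint handles only its spinning visuals, with no collection or boost logic.
; Tick rotates the whole actor in yaw and separately spins a central axis component, both at frame-rate-independent speeds.
; When IsGears is set, the construction script makes the axis and its children visible, and Tick also spins the individual gear components at their own rate.
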(event `self.ReceiveTick`
  (params (DeltaSeconds :type "Float (single-precision)"))
  (`self.K2_AddActorLocalRotation` (`KismetMathLibrary.MakeRotator` 0.0 0.0 (* DeltaSeconds (`self.Yaw/sec`))))
  ;[0.5569 0 1] Tony
  (`SceneComponent.K2_AddLocalRotation` (`self.Central Axis (Tony)`) (`KismetMathLibrary.MakeRotator` 0.0 0.0 (* DeltaSeconds (`self.Yaw/sec AllGears`))) false false)
  (if (`self.IsGears`)
    (`SceneComponent.K2_AddLocalRotation` (`self.Gears 3`) (`KismetMathLibrary.MakeRotator` 0.0 0.0 (* DeltaSeconds (`self.Yaw/sec Gears`))) false false)
    (`SceneComponent.K2_AddLocalRotation` (`self.Gears 2`) (`KismetMathLibrary.MakeRotator` 0.0 0.0 (* DeltaSeconds (`self.Yaw/sec Gears`))) false false)
    (`SceneComponent.K2_AddLocalRotation` (`self.Collectible_Gear_6`) (`KismetMathLibrary.MakeRotator` 0.0 0.0 (* DeltaSeconds (`self.Yaw/sec Gears`))) false false)
    (`SceneComponent.K2_AddLocalRotation` (`self.Collectible_Gear_7`) (`KismetMathLibrary.MakeRotator` 0.0 0.0 (* DeltaSeconds (`self.Yaw/sec Gears`))) false false)
    (`SceneComponent.K2_AddLocalRotation` (`self.Collectible_Gear_4`) (`KismetMathLibrary.MakeRotator` 0.0 0.0 (* DeltaSeconds (`self.Yaw/sec Gears`))) false false)
    (`SceneComponent.K2_AddLocalRotation` (`self.Gears 1`) (`KismetMathLibrary.MakeRotator` 0.0 0.0 (* DeltaSeconds (`self.Yaw/sec Gears`))) false false)
    (`SceneComponent.K2_AddLocalRotation` (`self.Collectible_Gear_2`) (`KismetMathLibrary.MakeRotator` 0.0 0.0 (* DeltaSeconds (`self.Yaw/sec Gears`))) false false)
    (`SceneComponent.K2_AddLocalRotation` (`self.Collectible_Gear_3`) (`KismetMathLibrary.MakeRotator` 0.0 0.0 (* DeltaSeconds (`self.Yaw/sec Gears`))) false false)
    (`SceneComponent.K2_AddLocalRotation` (`self.Collectible_Gear_5`) (`KismetMathLibrary.MakeRotator` 0.0 0.0 (* DeltaSeconds (`self.Yaw/sec Gears`))) false false)))

(fn `UserConstructionScript`
  (if (`self.IsGears`)
    (`SceneComponent.SetVisibility` (`self.Central Axis (Tony)`) true true)))